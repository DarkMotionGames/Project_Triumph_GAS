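; GA_FireBolt is a gameplay ability that casts a fire bolt at the point under the crosshair.
; On activation it takes the hit location from crosshair target data and sends it to the avatar as a facing warp target.
; It plays the cast-spell montage, spawns the projectile toward that location when the Firebolt montage event arrives, then ends after a short delay.
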(event `self.K2_ActivateAbility`
  (bind (_asynctaskproxy _datahandle) (`TargetDataUnderCrossHair.CreateTargetDataUnderCrossHair`)
    (:`ValidData`
      (set `self.ProjectileTargetLocation` (`.Location` (`GameplayStatics.BreakHitResult` (`AbilitySystemBlueprintLibrary.GetHitResultFromTargetData` _datahandle))))
      (message `CombatInterface.UpdateFacingWarpTarget` (`self.GetAvatarActorFromActorInfo`) (`self.ProjectileTargetLocation`))
      (`AbilityTask_PlayMontageAndWait.CreatePlayMontageAndWaitProxy` "None" "/Game/Assets/ControlRig/Characters/Mannequins/Animations/Manny/AM_CastSpell.AM_CastSpell" 1.2 "None" false
        (:`then`
          (`AbilityTask_WaitGameplayEvent.WaitGameplayEvent` (struct :`TagName` "Event.Montage.Firebolt") null
            (:`EventReceived`
              (`self.SpawnProjectile` (`self.ProjectileTargetLocation`))
              (`KismetSystemLibrary.Delay` 0.5)
              (`self.K2_EndAbility`))))))))