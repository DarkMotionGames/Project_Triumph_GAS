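; Enemy melee attack ability that plays a random attack montage from the avatar and damages live players near the striking socket.
; A looping timer keeps the motion-warping facing target on the enemy's combat target until the ability ends.
; The montage's gameplay event tag triggers the hit, selecting the combat socket for a small radius check that calls CauseDamage on each player found.
; The ability ends when the montage completes, is interrupted or is cancelled.
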(event `self.K2_ActivateAbility`
  (bind _returnvalue (`self.GetAvatarActorFromActorInfo`))
  (bind _returnvalue_2 (`self.GetAvatarActorFromActorInfo`))
  (bind _montage_tag (`self.Montage Tag`))
  (`|ExecutionSequence`
    (:`then_0`
      ; Init Variables
      (bind _asenemy_interface (cast `EnemyInterface` _returnvalue_2)
        (:`then`
          (set `self.CombatTarget` (`EnemyInterface.GetCombatTarget` _asenemy_interface))
          (bind _ascombat_interface (cast `CombatInterface` _returnvalue_2)
            (:`then`
              (set `self.Combat Interface` _ascombat_interface))
            (:`CastFailed`
              (`self.K2_EndAbility`))))
        (:`CastFailed`
          (`self.K2_EndAbility`))))
    (:`then_1`
      ; Play Anim Montage
      (bind (_montage _montage_tag_2) (`self.GetAnimMontageAndTag`))
      (set `self.Montage Tag` _montage_tag_2)
      (`AbilityTask_PlayMontageAndWait.CreatePlayMontageAndWaitProxy` "None" _montage
        (:`then`
          ; Timer For Motion Warping
          (bind _returnvalue_3 (`KismetSystemLibrary.K2_SetTimerDelegate` (delegate `OnSettingWarpTarget`) 0.01 true true))
          (set `self.TimeHandleSetFacingWarpTarget` _returnvalue_3)
          ; Apply Damage
          (`AbilityTask_WaitGameplayEvent.WaitGameplayEvent` _montage_tag null
            (:`EventReceived`
              (bind _returnvalue_4 (message `CombatInterface.GetCombatSocketLocation` _returnvalue _montage_tag))
              (bind _outoverlappingactors (`MainAbilitySystemLibrary.GetLivePlayersWithinRadius` _returnvalue (`|MakeArray` _returnvalue) 50.0 _returnvalue_4))
              (for _array_element _outoverlappingactors
                (`self.CauseDamage` _array_element)))))
        (:`OnCompleted`
          (`self.K2_EndAbility` :!label _label))
        (:`OnInterrupted`
          (goto _label))
        (:`OnCancelled`
          (goto _label))))))

(event `OnSettingWarpTarget`
  ; Timer For Motion Warping
  (`CombatInterface.UpdateFacingWarpTarget` (`self.Combat Interface`) (`Actor.K2_GetActorLocation` (`self.CombatTarget`))))

(event `self.K2_OnEndAbility`
  (params (bWasCancelled :type Boolean))
  ; End Ability
  (`KismetSystemLibrary.K2_ClearAndInvalidateTimerHandle` (`self.TimeHandleSetFacingWarpTarget`)))

(fn `GetAnimMontageAndTag`
  (returns (Montage :type "AnimMontage Object Reference") (`Montage Tag` :type "GameplayTag Structure"))
  (bind _returnvalue (message `CombatInterface.GetAttackMontage` (`self.GetAvatarActorFromActorInfo`)))
  (bind (_outitem _outindex) (`KismetArrayLibrary.Array_Random` _returnvalue))
  (if (> _outindex -1)
    (bind (_montage _montagetag) (break `TaggedMontage` _outitem))
    (return _montage _montagetag)
    (else
      (`self.K2_EndAbility`))))